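; BP_Shotgun is a shotgun that floats and spins as a pickup until the player character collects it.
; A timeline drives the bobbing, and overlapping the trigger resets the material, hands the gun to the character and stops the animation.
; Shooting checks cooldown and chamber, runs the parent's logic, reports a noise event and plays the shot sound.
; Alt-fire calls the upgrade logic.
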(event `self.Shoot`
  (bind _returnvalue (`self.GetOwner`))
  (if (and (`self.fireCooldown`) (> (`self.chamber`) 0))
    (`parent.Shoot`)
    (`AISense_Hearing.ReportNoiseEvent` (`self.K2_GetActorLocation` _returnvalue) (`self.noise`) _returnvalue)
    (`GameplayStatics.PlaySoundAtLocation` "/Game/Audio/Sound_Cue/SC_ShotgunShot.SC_ShotgunShot" (`self.K2_GetActorLocation`) (struct) 1.0 1.0 0.0 null null null null)))

(event `self.AltShoot`
  (`self.Upgrade`))

(event `self.ReceiveBeginPlay`
  (bind (_offset_location _offset_rotation _offset_scale) (`KismetMathLibrary.BreakTransform` (`self.Offset`)))
  (bind _output_get (set `self.StartPoint` (`self.K2_GetActorLocation`)))
  (bind (_direction _vertical_movement) (`Timeline|Timeline_0` :!via `PlayFromStart` :!label _label)
    (:`Update`
      (`self.K2_SetActorLocation` (+ _output_get (`KismetMathLibrary.MakeVector` 0.0 0.0 (* _vertical_movement 25.0))))
      (`SceneComponent.K2_AddLocalTransform` (`self.GunMesh`) (`KismetMathLibrary.MakeTransform` (0.0 0.0 0.0) (`KismetMathLibrary.MakeRotator` 0.0 (`self.Rotation Speed`)) _offset_scale) false false))))

(event `self.obtainGun.OnComponentBeginOverlap`
  (params (OverlappedComponent :type "PrimitiveComponent Object Reference") (OtherActor :type "Actor Object Reference") (OtherComp :type "PrimitiveComponent Object Reference") (OtherBodyIndex :type Integer) (bFromSweep :type Boolean) (SweepResult :type "HitResult Structure (by ref)"))
  (bind _asbp_third_person_character (cast `/Game/Blueprints/BP_ThirdPersonCharacter` OtherActor))
  (`/Engine/EditorBlueprintResources/StandardMacros.DoOnce` false
    (:`Completed`
      (`PrimitiveComponent.SetMaterial` (`self.GunMesh`) 0 "/Game/Models/Shotgun/defaultMat.defaultMat")
      (`/Game/Blueprints/BP_ThirdPersonCharacter.Add And Set Gun` _asbp_third_person_character self (`self.Offset`))
      (`PrimitiveComponent.SetCollisionEnabled` (`self.obtainGun`) "NoCollision")
      (goto _label :!via `Stop`))))

(fn `UserConstructionScript`)