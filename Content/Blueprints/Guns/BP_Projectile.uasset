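; BP_Projectile is an explosive projectile owned by BP_Gun_Projectile that detonates on a timer or on enemy contact.
; One tick after BeginPlay it copies Damage from the owning gun, then waits out its Timer before exploding.
; Sphere overlaps with BP_EnemyCharacter trigger detonation early, but only while the projectile is moving.
; Explode spawns a BP_Explosion carrying that damage, removes itself from the gun's GroupedBullets and destroys itself.
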(event `self.ReceiveBeginPlay`
  (`KismetSystemLibrary.DelayUntilNextTick`)
  (bind _asbp_gun_projectile (cast `/Game/Blueprints/Guns/BP_Gun_Projectile` (`self.GetOwner`)))
  (set `self.Damage` (`GunBaseClass.damage` _asbp_gun_projectile))
  (`KismetSystemLibrary.Delay` (`self.Timer`))
  (`self.Explode`)
  (`KismetSystemLibrary.PrintString` "Hello"))

(event `self.Sphere.OnComponentBeginOverlap`
  (params (OverlappedComponent :type "PrimitiveComponent Object Reference") (OtherActor :type "Actor Object Reference") (OtherComp :type "PrimitiveComponent Object Reference") (OtherBodyIndex :type Integer) (bFromSweep :type Boolean) (SweepResult :type "HitResult Structure (by ref)"))
  (if (and (== (`GameplayStatics.GetObjectClass` OtherActor) "/Game/Blueprints/Enemies/BP_EnemyCharacter.BP_EnemyCharacter_C") (!= (`MovementComponent.Velocity` (`self.ProjectileMovement`)) (0.0 0.0 0.0)))
    (`self.Explode`)))

(fn `Explode`
  (bind (_returnvalue_location _returnvalue_rotation) (`KismetMathLibrary.BreakTransform` (`self.GetTransform`)))
  (bind _returnvalue (`|SpawnActorFromClass` "/Game/Blueprints/Items/BP_Explosion.BP_Explosion_C" (`KismetMathLibrary.MakeTransform` _returnvalue_location _returnvalue_rotation) "Undefined" "OverrideRootScale" null null))
  (set `/Game/Blueprints/Items/BP_Explosion.Damage` (`self.Damage`) _returnvalue)
  (bind _asbp_gun_projectile (cast `/Game/Blueprints/Guns/BP_Gun_Projectile` (`self.GetOwner`)))
  (`KismetArrayLibrary.Array_RemoveItem` (`Gun_Projectile.groupedBullets` _asbp_gun_projectile) self)
  (`self.K2_DestroyActor`))

(fn `UserConstructionScript`)