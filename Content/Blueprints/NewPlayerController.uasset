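; Player controller that lets movement input interrupt pathfinding by repossessing the TargetCharacter.
; Unpossessing snapshots the movement axes, so only a non-zero input that differs from that snapshot beyond a threshold triggers possession.
; While another pawn is possessed, Tick moves it to the third-person character's follow camera and matches control rotation to that camera, maintaining the view during pathfinding.
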(event `self.ReceiveUnPossess`
  (params (UnpossessedPawn :type "Pawn Object Reference"))
  ;[1 1 1] Used to ensure changes in movement input interupt the player's pathfinding
  (set `self.PreviousInputs` (`KismetMathLibrary.MakeVector2D` (`self.GetInputAxisValue`) (`self.GetInputAxisValue`))))

(event `InputAxis|Move Forward / Backward` :consume false
  (params (AxisValue :type "Float (single-precision)"))
  (bind (_previousinputs_x _previousinputs_y) (`KismetMathLibrary.BreakVector2D` (`self.PreviousInputs`)))
  (bind _targetcharacter (`self.TargetCharacter`))
  ;[1 1 1] Used to ensure changes in movement input interupt the player's pathfinding
  (if (and (> (`KismetMathLibrary.Abs` (- AxisValue _previousinputs_y)) (`self.DeltaThreshold`)) (!= AxisValue 0.0))
    (if (and (`KismetSystemLibrary.IsValid` _targetcharacter) (!= (`GameplayStatics.GetPlayerCharacter` 0) _targetcharacter)) :!label _label
      (`self.Possess` (`self.TargetCharacter`)))))

(event `InputAxis|Move Right / Left` :consume false
  (params (AxisValue :type "Float (single-precision)"))
  (bind (_previousinputs_x _previousinputs_y) (`KismetMathLibrary.BreakVector2D` (`self.PreviousInputs`)))
  ;[1 1 1] Used to ensure changes in movement input interupt the player's pathfinding
  (if (and (> (`KismetMathLibrary.Abs` (- AxisValue _previousinputs_x)) (`self.DeltaThreshold`)) (!= AxisValue 0.0))
    (goto _label)))

(event `self.ReceiveTick`
  (params (DeltaSeconds :type "Float (single-precision)"))
  (bind _returnvalue (`self.K2_GetPawn`))
  (bind _targetcharacter (`self.TargetCharacter`))
  ;[1 1 1] Handle Camera While Pathfinding
  (if (and (!= _returnvalue _targetcharacter) (`KismetSystemLibrary.IsValid` _returnvalue))
    (bind _asbp_third_person_character (cast `/Game/Blueprints/BP_ThirdPersonCharacter` _targetcharacter))
    (bind _followcamera (`/Game/Blueprints/BP_ThirdPersonCharacter.FollowCamera` _asbp_third_person_character))
    (`self.K2_SetActorLocation` _returnvalue (`SceneComponent.K2_GetComponentLocation` _followcamera) false false)
    (`self.SetControlRotation` (`SceneComponent.K2_GetComponentRotation` _followcamera))))

(fn `UserConstructionScript`)