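; An EQS generator Blueprint that produces candidate cover points around the player character for enemy queries.
; It casts a ring of evenly spaced Visibility traces from Radius inward to the player's navmesh-projected location, so hits land on obstacle sides facing away from the player.
; Each hit is nudged out along its normal and raised, collected in LocationSet, then emitted as a generated vector.
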(fn `DoItemGeneration`
  (params (ContextLocations :type "Array of Vector Structure (by ref)"))
  (bind _projectedlocation (`NavigationSystemV1.K2_ProjectPointToNavigation` (`Actor.K2_GetActorLocation` (`GameplayStatics.GetPlayerCharacter` 0)) null "/Script/NavigationSystem.RecastFilter_UseDefaultArea"))
  (`KismetArrayLibrary.Array_Clear` (`self.LocationSet`))
  (for _index (range 36)
    (bind (_outhit _returnvalue) (`KismetSystemLibrary.LineTraceSingle` :`Start` (+ (* (`KismetMathLibrary.GreaterGreater_VectorRotator` (1.0 0.0 0.0) (`KismetMathLibrary.MakeRotator` 0.0 0.0 (* _index 10.0))) (`self.Radius`)) _projectedlocation) :`End` _projectedlocation :`TraceChannel` "TraceTypeQuery1" :`TraceColor` (struct :`R` 1.0 :`G` 0.739732 :`A` 1.0) :`TraceHitColor` (struct :`R` 1.0 :`G` 0.297748 :`A` 1.0)))
    (if _returnvalue
      (bind (_bblockinghit _binitialoverlap _time _distance _location _impactpoint _normal) (`GameplayStatics.BreakHitResult` _outhit))
      (`KismetArrayLibrary.Array_Add` (`self.LocationSet`) (+ _location (* _normal 10.0) (0.0 0.0 100.0)))))
  (for _array_element (`self.LocationSet`)
    (`self.AddGeneratedVector` _array_element))
  (return))