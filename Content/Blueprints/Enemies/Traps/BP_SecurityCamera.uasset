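; Security camera trap that sweeps back and forth and triggers an alarm when it detects the player's target character.
; Vision cone overlaps set visibility of the target, and Tick raises Awareness while seen or decays it more slowly otherwise.
; Full awareness fires the linked Alarm once and disables scanning and the cone, until ActivateTrap from the alarm restarts them.
; Sweep rotation uses a fixed per-frame step, not scaled by delta time.
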(event `self.ReceiveTick`
  (params (DeltaSeconds :type "Float (single-precision)"))
  ;[1 1 1] Awareness Behaviour
  (`|ExecutionSequence`
    (:`then_0`
      (if (`self.canSeePlayer`)
        (set `self.awareness` (`KismetMathLibrary.FClamp` (+ (`self.awareness`) (* DeltaSeconds 8.0)) 0.0 10.0))
        (else
          (set `self.awareness` (`KismetMathLibrary.FClamp` (- (`self.awareness`) (* DeltaSeconds 3.0)) 0.0 10.0)))))
    (:`then_1`
      (if (>= (`self.awareness`) 10.0)
        (`/Engine/EditorBlueprintResources/StandardMacros.DoOnce` false :!label _label
          (:`Completed`
            (`self.SoundAlarm`)))
        (else
          (goto _label :!via `Reset`))))
    (:`then_2`
      (if (`self.scanning`)
        (`self.Rotate`)))))

(event `StopScanning`
  (bind _visioncone (`self.VisionCone`))
  ;[1 1 1] Stop Scanning
  (set `self.scanning` false)
  (`PrimitiveComponent.SetCollisionEnabled` _visioncone "NoCollision")
  (`SceneComponent.SetVisibility` _visioncone false true))

(event `StartScanning`
  (bind _visioncone (`self.VisionCone`))
  ;[1 1 1] Start Scanning
  (set `self.scanning` true)
  (`PrimitiveComponent.SetCollisionEnabled` _visioncone "QueryOnly")
  (`SceneComponent.SetVisibility` _visioncone true true)
  (set `self.canSeePlayer` false))

(event `self.VisionCone.OnComponentBeginOverlap`
  (params (OverlappedComponent :type "PrimitiveComponent Object Reference") (OtherActor :type "Actor Object Reference") (OtherComp :type "PrimitiveComponent Object Reference") (OtherBodyIndex :type Integer) (bFromSweep :type Boolean) (SweepResult :type "HitResult Structure (by ref)"))
  ;[1 1 1] Is the player within the camera's vision cone?
  (if (== OtherActor (`self.Target`))
    (set `self.canSeePlayer` true)))

(event `Rotate`
  (bind _rotationspeed (`self.rotationSpeed`))
  (bind _rotationspeed_2 (`self.rotationSpeed`))
  ;[1 1 1] Rotation
  (if (`self.rotatingRight`)
    (set `self.degreesRemaining` (- (`self.degreesRemaining`) _rotationspeed))
    (`self.K2_AddActorLocalRotation` (`KismetMathLibrary.MakeRotator` 0.0 0.0 (* _rotationspeed -1.0)))
    (if (<= (`self.degreesRemaining`) (* (`self.maxRotationAngle`) -1.0))
      (set `self.rotatingRight` false))
    (else
      (set `self.degreesRemaining` (+ (`self.degreesRemaining`) _rotationspeed_2))
      (`self.K2_AddActorLocalRotation` (`KismetMathLibrary.MakeRotator` 0.0 0.0 _rotationspeed_2))
      (if (>= (`self.degreesRemaining`) (`self.maxRotationAngle`))
        (set `self.rotatingRight` true)))))

(event `self.VisionCone.OnComponentEndOverlap`
  (params (OverlappedComponent :type "PrimitiveComponent Object Reference") (OtherActor :type "Actor Object Reference") (OtherComp :type "PrimitiveComponent Object Reference") (OtherBodyIndex :type Integer))
  ;[1 1 1] Is the player within the camera's vision cone?
  (if (== OtherActor (`self.Target`))
    (set `self.canSeePlayer` false)))

(event `ActivateTrap`
  ;[1 1 1] Activate Trap (Called by alarm)
  (if (not (`self.scanning`))
    (`self.StartScanning`)))

(event `SoundAlarm`
  ;[1 1 1] Sound the alarm
  (`self.StopScanning`)
  (`/Game/Blueprints/Enemies/Traps/BP_Alarm.ActivateAlarm` (`self.alarm`)))

(event `self.ReceiveBeginPlay`
  ;[1 1 1] Cache reference to our target character
  (`KismetSystemLibrary.DelayUntilNextTick`)
  (bind _asnew_player_controller (cast `/Game/Blueprints/NewPlayerController` (`GameplayStatics.GetPlayerController` 0)))
  (set `self.Target` (`/Game/Blueprints/NewPlayerController.TargetCharacter` _asnew_player_controller)))

(fn `UserConstructionScript`)