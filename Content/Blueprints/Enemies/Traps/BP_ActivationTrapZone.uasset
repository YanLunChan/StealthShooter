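; Trap zone that fires an array of linked traps in sequence while the third-person character is inside its Activation volume.
; Entering starts a self-repeating delay loop that calls TriggerTrapMessage through the Triggerable interface on one trap per pass, wrapping the index.
; Exiting clears Attack and sends that state to every trap.
; The delay loop itself keeps running afterwards, only resetting the index.
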(event `self.activation.OnComponentBeginOverlap`
  (params (OverlappedComponent :type "PrimitiveComponent Object Reference") (OtherActor :type "Actor Object Reference") (OtherComp :type "PrimitiveComponent Object Reference") (OtherBodyIndex :type Integer) (bFromSweep :type Boolean) (SweepResult :type "HitResult Structure (by ref)"))
  (cast `/Game/Blueprints/BP_ThirdPersonCharacter` OtherActor)
  (`KismetSystemLibrary.PrintString` "Activated")
  (set `self.attack` true)
  (`self.Loop` :!label _label)
  (`KismetSystemLibrary.Delay` (`self.delay`))
  (goto _label))

(event `self.activation.OnComponentEndOverlap`
  (params (OverlappedComponent :type "PrimitiveComponent Object Reference") (OtherActor :type "Actor Object Reference") (OtherComp :type "PrimitiveComponent Object Reference") (OtherBodyIndex :type Integer))
  (cast `/Game/Blueprints/BP_ThirdPersonCharacter` OtherActor)
  (`KismetSystemLibrary.PrintString` "Deactivated")
  (bind _output_get (set `self.attack` false))
  (for _array_element (`self.Traps`)
    (message `/Game/Blueprints/Enemies/Traps/Triggerable.TriggerTrap` _array_element _output_get)))

(fn `Loop`
  (bind _attack (`self.attack`))
  (bind _traps (`self.Traps`))
  (bind _index (`self.index`))
  (bind _output (`|GetArrayItem` _traps _index))
  (if (and _attack (`KismetSystemLibrary.DoesImplementInterface` _output "/Game/Blueprints/Enemies/Traps/Triggerable.Triggerable_C"))
    (message `/Game/Blueprints/Enemies/Traps/Triggerable.TriggerTrap` _output _attack)
    (if (< _index (`KismetArrayLibrary.Array_Length` _traps))
      (`/Engine/EditorBlueprintResources/StandardMacros.IncrementInt` (`self.index`))
      (else
        (set `self.index` 0 :!label _label)))
    (else
      (goto _label))))

(fn `UserConstructionScript`)