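; BP_SawWallTrap is a trap with a spinning saw that shuttles between two points and damages the player on contact.
; BeginPlay caches the actor's location and the End component's world location as the endpoints.
; Tick spins the Cylinder per frame and lerps the actor between them over Time, with a FlipFlop reversing direction.
; Box overlap applies Damage to actors matching the player character's exact class.
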(event `self.ReceiveBeginPlay`
  (set `self.Start Point` (`self.K2_GetActorLocation`))
  (set `self.End Point` (`SceneComponent.K2_GetComponentLocation` (`self.End`))))

(event `self.ReceiveTick`
  (params (DeltaSeconds :type "Float (single-precision)"))
  (bind _end_point (`self.End Point`))
  (bind _start_point (`self.Start Point`))
  (bind _returnvalue (/ (`self.Count`) (`self.Time`)))
  ;[1 1 1] Spin the saw
  (`SceneComponent.K2_AddLocalRotation` (`self.Cylinder`) (`KismetMathLibrary.MakeRotator` 0.0 0.0 (`self.Rotation Speed`)) false false)
  ;[1 1 1] Go to
  (if (`self.To End?`)
    (`self.K2_SetActorLocation` (`KismetMathLibrary.VLerp` _start_point _end_point _returnvalue))
    (else
      (`self.K2_SetActorLocation` (`KismetMathLibrary.VLerp` _end_point _start_point _returnvalue))))
  (bind _output_get (set `self.Count` (+ (`self.Count`) DeltaSeconds)))
  (if (> _output_get (`self.Time`))
    (set `self.Count` 0.0)
    (`/Engine/EditorBlueprintResources/StandardMacros.FlipFlop`
      (:`A`
        (set `self.To End?` false))
      (:`B`
        (set `self.To End?` true)))))

(event `self.Box.OnComponentBeginOverlap`
  (params (OverlappedComponent :type "PrimitiveComponent Object Reference") (OtherActor :type "Actor Object Reference") (OtherComp :type "PrimitiveComponent Object Reference") (OtherBodyIndex :type Integer) (bFromSweep :type Boolean) (SweepResult :type "HitResult Structure (by ref)"))
  (if (== (`GameplayStatics.GetObjectClass` OtherActor) (`GameplayStatics.GetObjectClass` (`GameplayStatics.GetPlayerCharacter` 0)))
    (`GameplayStatics.ApplyDamage` OtherActor (`self.Damage`))))

(fn `UserConstructionScript`)