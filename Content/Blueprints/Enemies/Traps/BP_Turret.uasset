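; BP_Turret is a trap turret that tracks the player controller's target character and shoots projectiles when triggered.
; TriggerTrap toggles activation, and Tick rotates the head at constant speed toward the target, or back to its starting rotation when inactive.
; UpdateFire fires once the cooldown has elapsed and a dot product confirms alignment.
; Fire uses a self-re-entering DoN with a delay to spawn two-shot bursts of BP_Trap_Proj.
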(event `self.ReceiveBeginPlay`
  (set `self.Starting Rotation` (`self.K2_GetActorRotation`))
  (`KismetSystemLibrary.DelayUntilNextTick`)
  (bind _asnew_player_controller (cast `/Game/Blueprints/NewPlayerController` (`GameplayStatics.GetPlayerController` 0)))
  (set `self.Target` (`/Game/Blueprints/NewPlayerController.TargetCharacter` _asnew_player_controller)))

(event `self.ReceiveTick`
  (params (DeltaSeconds :type "Float (single-precision)"))
  (bind _turret_head (`self.Turret Head`))
  (bind _interp_speed (`self.Interp Speed`))
  (bind _returnvalue (`SceneComponent.K2_GetComponentRotation` _turret_head))
  (if (`self.Activated`)
    (`self.Rotate Update` (`KismetMathLibrary.RInterpTo_Constant` _returnvalue (`KismetMathLibrary.FindLookAtRotation` (`SceneComponent.K2_GetComponentLocation` _turret_head) (`self.K2_GetActorLocation` (`self.Target`))) DeltaSeconds _interp_speed))
    (`self.Update Fire`)
    (else
      (`self.Rotate Update` (`KismetMathLibrary.RInterpTo_Constant` _returnvalue (`self.Starting Rotation`) DeltaSeconds _interp_speed)))))

(event `/Game/Blueprints/Enemies/Traps/Triggerable.TriggerTrap`
  (params (Attack :type Boolean))
  (set `self.Activated` Attack))

(event `Fire`
  (set `self.LastFireT` (`KismetSystemLibrary.GetGameTimeInSeconds`))
  (`|ExecutionSequence`
    (:`then_0`
      (goto _label :!via `Reset`))
    (:`then_1`
      (`/Engine/EditorBlueprintResources/StandardMacros.Do N` 2 :!label _label
        (:`Exit`
          (`|SpawnActorFromClass` "/Game/Blueprints/Enemies/Traps/BP_Trap_Proj.BP_Trap_Proj_C" (`KismetMathLibrary.MakeTransform` (`SceneComponent.K2_GetComponentLocation` (`self.Muzzle Local`)) (`SceneComponent.K2_GetComponentRotation` (`self.Turret Head`)) (0.25 0.25 0.25)) "Undefined" "OverrideRootScale" null null)
          (`KismetSystemLibrary.Delay` 0.2)
          (goto _label))))))

(fn `Rotate Update`
  (params (Rotation :type "Rotator Structure"))
  (`SceneComponent.K2_SetWorldRotation` (`self.Turret Head`) Rotation false false))

(fn `Update Fire`
  (bind _turret_head (`self.Turret Head`))
  (if (and (> (- (`KismetSystemLibrary.GetGameTimeInSeconds`) (`self.LastFireT`)) (`self.Rate of Fire`)) (> (`KismetMathLibrary.Dot_VectorVector` (`KismetMathLibrary.GetDirectionUnitVector` (`SceneComponent.K2_GetComponentLocation` _turret_head) (`self.K2_GetActorLocation` (`self.Target`))) (`SceneComponent.GetForwardVector` _turret_head)) 0.99))
    (`self.Fire`)))

(fn `UserConstructionScript`)