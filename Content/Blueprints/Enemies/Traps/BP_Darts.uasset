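; BP_Darts is a dart trap that fires projectiles from three muzzle points when triggered.
; The TriggerTrap event, when its Attack flag is true, passes the world transforms of the three muzzles to SpawnProj.
; SpawnProj loops over them and spawns a scaled-down BP_Trap_Proj at each, nudged clear of collisions if possible but always spawned.
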(event `/Game/Blueprints/Enemies/Traps/Triggerable.TriggerTrap`
  (params (Attack :type Boolean))
  (if Attack
    (`self.Spawn Proj` (`|MakeArray` (`SceneComponent.K2_GetComponentToWorld` (`self.Muzzle 1`)) (`SceneComponent.K2_GetComponentToWorld` (`self.Muzzle 2`)) (`SceneComponent.K2_GetComponentToWorld` (`self.Muzzle 3`))))))

(fn `Spawn Proj`
  (params (Transform :type "Array of Transform Structure"))
  (for _array_element Transform
    (`|SpawnActorFromClass` "/Game/Blueprints/Enemies/Traps/BP_Trap_Proj.BP_Trap_Proj_C" (`KismetMathLibrary.MakeTransform` (.location _array_element) (.rotation _array_element) (0.25 0.25 0.25)) "AdjustIfPossibleButAlwaysSpawn" "OverrideRootScale" null null)))

(fn `UserConstructionScript`)