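; BP_Alarm is a trap-triggered alarm that shows a rotating spotlight and alerts the game to the player's target character.
; Activation reports a noise at the target's location with the alarm as instigator and notifies the character it tripped the alarm.
; A 30-second retriggerable delay then switches the alarm off and reactivates linked security camera and laser traps.
; The target is cached from the player controller one tick after BeginPlay.
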(event `self.ReceiveTick`
  (params (DeltaSeconds :type "Float (single-precision)"))
  ;[1 1 1] Rotate Light
  (if (`self.alarmActivated`)
    (`SceneComponent.K2_AddWorldRotation` (`self.SpotLight`) (struct :`Yaw` 2.0) false false)))

(event `ActivateAlarm`
  ;[1 1 1] Activate alarm (Called by trap)
  (set `self.alarmActivated` true)
  (`SceneComponent.SetVisibility` (`self.SpotLight`) true false)
  (`AISense_Hearing.ReportNoiseEvent` (`self.K2_GetActorLocation` (`self.Target`)) 2.0 self)
  (`|ExecutionSequence`
    (:`then_0`
      (bind _asbp_third_person_character (cast `/Game/Blueprints/BP_ThirdPersonCharacter` (`self.Target`)))
      (`/Game/Blueprints/BP_ThirdPersonCharacter.TrippedAlarm` _asbp_third_person_character))
    (:`then_1`
      (`KismetSystemLibrary.RetriggerableDelay` 30.0)
      (`self.DeactivateAlarm`))))

(event `DeactivateAlarm`
  ;[1 1 1] Deactivate alarm
  (set `self.alarmActivated` false)
  (`SceneComponent.SetVisibility` (`self.SpotLight`) false false)
  (for _array_element (`self.traps`)
    (bind _asbp_security_camera (cast `/Game/Blueprints/Enemies/Traps/BP_SecurityCamera` _array_element) ; If the trap is a security camera
      (:`then`
        (`/Game/Blueprints/Enemies/Traps/BP_SecurityCamera.ActivateTrap` _asbp_security_camera))
      (:`CastFailed`
        (bind _asbp_laser (cast `/Game/Blueprints/Enemies/Traps/BP_Laser` _array_element)) ; If the trap is a laser
        (`/Game/Blueprints/Enemies/Traps/BP_Laser.ActivateTrap` _asbp_laser)))))

(event `self.ReceiveBeginPlay`
  ;[1 1 1] Cache Reference to our target character
  (`KismetSystemLibrary.DelayUntilNextTick`)
  (bind _asnew_player_controller (cast `/Game/Blueprints/NewPlayerController` (`GameplayStatics.GetPlayerController` 0)))
  (set `self.Target` (`/Game/Blueprints/NewPlayerController.TargetCharacter` _asnew_player_controller)))

(fn `UserConstructionScript`)