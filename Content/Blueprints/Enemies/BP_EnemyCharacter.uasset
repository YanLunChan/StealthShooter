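; Enemy AI character that patrols, investigates noises and hunts the player through a graded awareness meter, then attacks and dies in ragdoll.
; AI Perception sight and hearing drive awareness, which rises faster at close range, decays when idle and updates a color-coded bar facing the player.
; Awareness thresholds set movement speed and blackboard keys for approach, attack, firing position and destination.
; Shooting uses spread line traces with Niagara tracers, noise reports and blackboard-tracked ammo.
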(event `self.ReceiveBeginPlay`
  ;[1 1 1] Initialization
  (`KismetSystemLibrary.DelayUntilNextTick`)
  (bind _asnew_player_controller (cast `/Game/Blueprints/NewPlayerController` (`GameplayStatics.GetPlayerController` 0)))
  (set `self.Target` (`/Game/Blueprints/NewPlayerController.TargetCharacter` _asnew_player_controller))
  (set `CharacterMovementComponent.MaxWalkSpeed` (`self.walkSpeed`) (`self.CharacterMovement`))
  (`BlackboardComponent.SetValueAsInt` (`AIBlueprintHelperLibrary.GetBlackboard` null) "RemainingBullets" (`self.maxBullets`))
  (bind _asbp_enemy_awareness (cast `/Game/Blueprints/UI/BP_EnemyAwareness` (`WidgetComponent.GetWidget` (`self.AwarenessWidget`))))
  (set `self.AwarenessProgressBar` (`/Game/Blueprints/UI/BP_EnemyAwareness.ProgressBar_174` _asbp_enemy_awareness))
  (bind _asbp_my_game_instance (cast `/Game/Blueprints/BP_MyGameInstance` (`GameplayStatics.GetGameInstance`)))
  (set `self.gameInstance` _asbp_my_game_instance)
  (`KismetSystemLibrary.Delay` 0.5)
  (bind _asbp_third_person_character (cast `/Game/Blueprints/BP_ThirdPersonCharacter` (`self.Target`)))
  (bind _result (`/Game/Blueprints/UI/Minimap/MinimapWidget.AddArrow` (`/Game/Blueprints/UI/BP_Hud.MinimapWidget` (`/Game/Blueprints/BP_ThirdPersonCharacter.Hud REF` _asbp_third_person_character)) false (make `Color` 1 0 0 1) self))
  (set `self.Arrow` _result))

(event `LookAtPlayer`
  (bind (_returnvalue_roll _returnvalue_pitch _returnvalue_yaw) (`KismetMathLibrary.BreakRotator` (`KismetMathLibrary.FindLookAtRotation` (`self.K2_GetActorLocation`) (`self.K2_GetActorLocation` (`self.Target`)))))
  ;[1 1 1] Look at the Player
  (`self.K2_SetActorRotation` (`KismetMathLibrary.MakeRotator` 0.0 0.0 _returnvalue_yaw)))

(event `self.ReceiveTick`
  (params (DeltaSeconds :type "Float (single-precision)"))
  (bind _returnvalue (`AIBlueprintHelperLibrary.GetBlackboard` null))
  (bind _returnvalue_2 (`AIBlueprintHelperLibrary.GetBlackboard` null))
  (bind _returnvalue_3 (`self.K2_GetActorLocation`))
  (bind _awareness (`self.awareness`))
  (bind _awareness_2 (`self.awareness`))
  (bind _returnvalue_4 (`self.K2_GetActorLocation` (`self.Target`)))
  (bind _returnvalue_5 (`KismetMathLibrary.Vector_Distance` (`self.K2_GetActorLocation`) (`self.K2_GetActorLocation` (`self.Target`))))
  ;[1 1 1] On Tick
  (`|ExecutionSequence`
    (:`then_0`
      ;[1 1 1] Are we attacking the player?
      (if (`self.isDead`)
        _
        (elif (== _awareness 10.0)
          (`|ExecutionSequence`
            (:`then_0`
              (`/Engine/EditorBlueprintResources/StandardMacros.DoOnce` false
                (:`Completed`
                  (`BlackboardComponent.SetValueAsBool` (`AIBlueprintHelperLibrary.GetBlackboard` null) "Attacking" true)
                  (set `CharacterMovementComponent.MaxWalkSpeed` (`self.runSpeed`) (`self.CharacterMovement`))
                  (`/Game/Blueprints/BP_MyGameInstance.EnemyStartsChasing` (`self.gameInstance`))
                  (`KismetSystemLibrary.PrintString` "Start chasing"))))
            (:`then_1`
              (bind _outhit (`KismetSystemLibrary.LineTraceSingleForObjects` _returnvalue_3 _returnvalue_4 (`self.Object Types`)))
              (if (and (<= (`KismetMathLibrary.Vector_Distance` _returnvalue_3 _returnvalue_4) (`self.maxFireRange`)) (== (`.HitActor` (`GameplayStatics.BreakHitResult` _outhit)) (`self.Target`)))
                (`BlackboardComponent.SetValueAsBool` _returnvalue "InPosition" true)
                (else
                  (`BlackboardComponent.SetValueAsBool` _returnvalue "InPosition" false))))
            (:`then_2`
              (if (`self.canSeePlayer`)
                (`self.LookAtPlayer`))))
          (else
            ;[1 1 1] Awareness Behavior
            (if (`self.canSeePlayer`)
              (`self.LookAtPlayer`)
              (if (< _returnvalue_5 500.0)
                (set `self.awareness` 10.0) ; Start attacking
                (`self.UpdateAwarenessUI`)
                (`GameplayStatics.PlaySoundAtLocation` "/Game/Audio/Sound_Cue/Sound_Clip/Alert.Alert" (`self.K2_GetActorLocation`) (struct) 1.0 1.0 0.0 null null null null)
                (else
                  (bind _output_get (set `self.awareness` (`KismetMathLibrary.FClamp` (+ _awareness_2 (/ (* DeltaSeconds 2000.0) _returnvalue_5)) 0.0 10.0))) ; Raise awareness
                  (`self.UpdateAwarenessUI`)
                  (if (> _output_get 5.0)
                    (`BlackboardComponent.SetValueAsBool` _returnvalue_2 "ApproachingPlayer" true) ; Approach Player
                    (`BlackboardComponent.SetValueAsObject` _returnvalue_2 "PlayerReference" (`self.Target`)) ; Set player location in BB
                    (if (>= (`self.awareness`) 6.0)
                      (`/Engine/EditorBlueprintResources/StandardMacros.DoOnce` false :!label _label
                        (:`Completed`
                          (set `CharacterMovementComponent.MaxWalkSpeed` (`self.runSpeed`) (`self.CharacterMovement`))))))))
              (elif (not (`self.investigating`))
                (set `self.awareness` (`KismetMathLibrary.FClamp` (- _awareness_2 DeltaSeconds) 0.0 10.0)) ; Lower awareness
                (`self.UpdateAwarenessUI`)
                (`BlackboardComponent.SetValueAsBool` _returnvalue_2 "ApproachingPlayer" false) ; Stop approaching Player
              ))))))
    (:`then_1`
      (if (> _awareness 0.0)
        (`SceneComponent.K2_SetWorldRotation` (`self.AwarenessWidget`) (`KismetMathLibrary.FindLookAtRotation` (`SceneComponent.K2_GetComponentLocation` (`self.AwarenessWidget`)) (`self.K2_GetActorLocation` (`self.Target`))) false false)))))

(event `SpawnBulletTracer`
  (params (BeamEnd :type "Vector Structure"))
  ;[1 1 1] Spawn Bullet Tracers
  (bind _returnvalue (`NiagaraFunctionLibrary.SpawnSystemAtLocation` "/Game/Effects/N_Tracer_System.N_Tracer_System" (`SceneComponent.K2_GetComponentLocation` (`self.Gun`))))
  (`FXSystemComponent.SetVectorParameter` _returnvalue "BeamEnd" BeamEnd))

(event `Reached Destination`
  (bind _patrolpoints (`self.patrolPoints`))
  ;[1 1 1] Reached Destination
  (set `self.investigating` false)
  (set `CharacterMovementComponent.MaxWalkSpeed` (`self.walkSpeed`) (`self.CharacterMovement`))
  (`BlackboardComponent.SetValueAsVector` (`AIBlueprintHelperLibrary.GetBlackboard` null) "Destination" (`self.K2_GetActorLocation` (`|GetArrayItem` _patrolpoints (`KismetMathLibrary.RandomIntegerInRange` 0 (- (`KismetArrayLibrary.Array_Length` _patrolpoints) 1)))))
  (goto _label :!via `Reset`))

(event `Shoot`
  (bind _returnvalue (`AIBlueprintHelperLibrary.GetBlackboard` null))
  (bind _firingspread (`self.firingSpread`))
  (bind _target (`self.Target`))
  (bind (_returnvalue_x _returnvalue_y _returnvalue_z) (`KismetMathLibrary.BreakVector` (`self.K2_GetActorLocation` (`self.Target`))))
  (bind _returnvalue_2 (`SceneComponent.K2_GetComponentLocation` (`self.Gun`)))
  (bind _returnvalue_3 (* _firingspread 0.5))
  (bind _returnvalue_4 (* _firingspread -0.5))
  ;[1 1 1] Shoot at Player
  (bind _result (`/Engine/EditorBlueprintResources/StandardMacros.DecrementInt` (`BlackboardComponent.GetValueAsInt` _returnvalue "RemainingBullets"))
    (:`  `
      (`BlackboardComponent.SetValueAsInt` _returnvalue "RemainingBullets" _result)
      (bind _output_get (set `self.firingTarget` (+ _returnvalue_2 (* (`KismetMathLibrary.Normal` (`KismetMathLibrary.GreaterGreater_VectorRotator` (- (`KismetMathLibrary.MakeVector` _returnvalue_x _returnvalue_y (+ _returnvalue_z (* (`CapsuleComponent.CapsuleHalfHeight` (`self.CapsuleComponent`)) 0.5))) _returnvalue_2) (`KismetMathLibrary.MakeRotator` 0.0 (`KismetMathLibrary.RandomFloatInRange` _returnvalue_4 _returnvalue_3) (`KismetMathLibrary.RandomFloatInRange` _returnvalue_4 _returnvalue_3)))) (`self.maxFireRange`) 2.0))))
      (`KismetSystemLibrary.Delay` 0.1)
      (bind _outhit (`KismetSystemLibrary.LineTraceSingle` :`Start` _returnvalue_2 :`End` _output_get :`TraceChannel` "TraceTypeQuery3" :`TraceColor` (struct :`R` 0.088937 :`B` 1.0 :`A` 1.0)))
      (`self.SpawnBulletTracer` (`.Location` (`GameplayStatics.BreakHitResult` _outhit)))
      (`AISense_Hearing.ReportNoiseEvent` (`self.K2_GetActorLocation`) 2.5 self)
      (if (== (`.HitActor` (`GameplayStatics.BreakHitResult` _outhit)) _target)
        (`KismetSystemLibrary.PrintString` "Hit Player")
        (bind _asbp_third_person_character (cast `/Game/Blueprints/BP_ThirdPersonCharacter` _target))
        (`GameplayStatics.ApplyDamage` _asbp_third_person_character 20.0 null self "/Script/Engine.DamageType")))))

(event `self.AIPerception.OnPerceptionUpdated`
  (params (UpdatedActors :type "Array of Actor Object Reference (by ref)"))
  ;[1 1 1] On Perception Updated
  (if (not (`self.isDead`))
    (for _array_element UpdatedActors
      (bind _info (`AIPerceptionComponent.GetActorsPerception` (`self.AIPerception`) _array_element))
      (for (_array_element_2 _array_index) (`.LastSensedStimuli` (break `ActorPerceptionBlueprintInfo` _info))
        (if (and (== _array_index 0) (== (break `ActorPerceptionBlueprintInfo` _info) (`self.Target`)))
          ;[1 1 1] Update Player's Visibility Status
          (if (`.bSuccessfullySensed` (break `AIStimulus` _array_element_2))
            (set `self.canSeePlayer` true)
            (else
              (set `self.canSeePlayer` false) ; Lost sight of player
              (if (> (`self.awareness`) 5.0)
                (`BlackboardComponent.SetValueAsVector` (`AIBlueprintHelperLibrary.GetBlackboard` null) "Destination" (`self.K2_GetActorLocation` (`self.Target`))) ; Check player's last known location
              )))
          (elif (and (== _array_index 1) (`.bSuccessfullySensed` (break `AIStimulus` _array_element_2)))
            ;[1 1 1] Heard A Sound
            (`self.Alert` (`.Strength` (break `AIStimulus` _array_element_2)) (`.StimulusLocation` (break `AIStimulus` _array_element_2)))))))))

(event `Alert`
  (params (noiseLoudness :type "Float (double-precision)") (noiseLocation :type "Vector Structure"))
  (bind _awareness (`self.awareness`))
  ;[1 1 1] Alert (Reaction to noises and distractions)
  (if (>= noiseLoudness (`self.currentLoudness`))
    (set `self.investigating` true)
    (`BlackboardComponent.SetValueAsVector` (`AIBlueprintHelperLibrary.GetBlackboard` null) "Destination" noiseLocation) ; Check noise location
    (bind _output_get (set `self.currentLoudness` noiseLoudness))
    (if (< _output_get 2.0)
      (if (< _awareness 5.0)
        (set `self.awareness` 5.0) ; Running & Distractions
        (`self.UpdateAwarenessUI` :!label _label_2))
      (elif (< _awareness 6.0)
        (set `self.awareness` 6.0) ; Traps & Shooting
        (set `CharacterMovementComponent.MaxWalkSpeed` (`self.runSpeed`) (`self.CharacterMovement`))
        (goto _label_2)))))

(event `self.ReceiveAnyDamage`
  (params (Damage :type "Float (single-precision)") (DamageType :type "DamageType Object Reference") (InstigatedBy :type "Controller Object Reference") (DamageCauser :type "Actor Object Reference"))
  (bind _returnvalue (`self.K2_GetActorLocation`))
  (bind _health (`self.Health`))
  (bind _arrow (`self.Arrow`))
  ;[1 1 1] Take Damage / Death
  (`HealthComponent.TakeDamage` _health null Damage DamageType InstigatedBy DamageCauser)
  (if (<= (`HealthComponent.health` _health) 0.0)
    (set `self.isDead` true)
    (`self.DetachFromControllerPendingDestroy`)
    (`GameplayStatics.PlaySoundAtLocation` "/Game/Audio/Sound_Cue/Sound_Clip/Man_Death.Man_Death" _returnvalue (struct) 1.0 1.0 0.0 null null null null)
    (`PrimitiveComponent.SetSimulatePhysics` (`self.Mesh`) true)
    (`PrimitiveComponent.SetCollisionEnabled` (`self.CapsuleComponent`) "NoCollision")
    (`/Game/Blueprints/BP_MyGameInstance.EnemyStopsChasing` (`self.gameInstance`))
    (`KismetSystemLibrary.Delay` 5.0)
    (`self.K2_DestroyActor`)
    (`/Engine/EditorBlueprintResources/StandardMacros.IsValid` _arrow
      (:`Is Valid`
        (`Widget.RemoveFromParent` _arrow)))
    (else
      (`GameplayStatics.PlaySoundAtLocation` "/Game/Audio/Sound_Cue/Sound_Clip/Man_Hurt.Man_Hurt" _returnvalue (struct) 1.0 1.0 0.0 null null null null))))

(event `Reload`
  ;[1 1 1] Reload
  (`|PlayMontage` (`self.Mesh`) "/Game/Animation/GunPoses/PistolReloadAM.PistolReloadAM"
    (:`OnCompleted`
      (`BlackboardComponent.SetValueAsInt` (`AIBlueprintHelperLibrary.GetBlackboard` null) "RemainingBullets" (`self.maxBullets`))
      (`KismetSystemLibrary.PrintString` "Reloading"))))

(event `UpdateAwarenessUI`
  (bind _awareness (`self.awareness`))
  (bind _awarenessprogressbar (`self.AwarenessProgressBar`))
  (bind _awarenessprogressbar_2 (`self.AwarenessProgressBar`))
  ;[1 1 1] Update Awareness UI
  (`/Engine/EditorBlueprintResources/StandardMacros.IsValid` _awarenessprogressbar
    (:`Is Valid`
      (`ProgressBar.SetPercent` _awarenessprogressbar (/ _awareness 10.0))
      (if (<= _awareness 0.0)
        (`Widget.SetVisibility` _awarenessprogressbar "Hidden")
        (else
          (`Widget.SetVisibility` _awarenessprogressbar "Visible")
          (if (< (`self.awareness`) 6.0)
            (`ProgressBar.SetFillColorAndOpacity` _awarenessprogressbar_2 (struct :`R` 1.0 :`G` 0.908744 :`A` 1.0))
            (elif (< (`self.awareness`) 10.0)
              (`ProgressBar.SetFillColorAndOpacity` _awarenessprogressbar_2 (struct :`R` 1.0 :`G` 0.342601 :`A` 1.0))
              (else
                (`ProgressBar.SetFillColorAndOpacity` _awarenessprogressbar_2 (struct :`R` 0.833333 :`A` 1.0))))))))))

(fn `UserConstructionScript`)