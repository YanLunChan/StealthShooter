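; Game instance Blueprint that manages background music, switching between slow and fast tracks depending on whether enemies are chasing the player.
; Chase start and stop events keep a count of chasing enemies, switching to fast music on the first chaser and slow music when none remain.
; A single stored 2D audio component, created by PlayAudio with optional persistence across level transitions, has its sound swapped by ChangeAudio and is halted by StopAudio.
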(event `EnemyStartsChasing`
  (`/Engine/EditorBlueprintResources/StandardMacros.IncrementInt` (`self.enemiesChasing`)
    (:`  `
      (if (not (`self.beingChased`))
        (set `self.beingChased` true)
        (`self.ChangeAudio` "/Game/Audio/FastMusic.FastMusic")))))

(event `EnemyStopsChasing`
  (bind _result (`/Engine/EditorBlueprintResources/StandardMacros.DecrementInt` (`self.enemiesChasing`))
    (:`  `
      (if (<= _result 0)
        (set `self.beingChased` false)
        (`self.ChangeAudio` "/Game/Audio/SlowMusic.SlowMusic")))))

(event `StopAudio`
  (bind _music (`self.Music`))
  (`/Engine/EditorBlueprintResources/StandardMacros.IsValid` _music
    (:`Is Valid`
      (`AudioComponent.Stop` _music))))

(fn `ChangeAudio`
  (params (NewSound :type "SoundBase Object Reference"))
  (`AudioComponent.SetSound` (`self.Music`) NewSound))

(fn `PlayAudio`
  (params (Sound :type "SoundBase Object Reference") (VolumeMultiplier :type "Float (single-precision)") (bPersistAcrossLevelTransition :type Boolean))
  (bind _returnvalue (`GameplayStatics.CreateSound2D` Sound VolumeMultiplier 1.0 0.0 null bPersistAcrossLevelTransition))
  (bind _output_get (set `self.Music` _returnvalue))
  (`AudioComponent.Play` _output_get 0.0))