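; BP_PlantSite is a bomb plant objective, marked in the world by a bouncing cone and on the minimap by a static arrow.
; A timeline animates the cone, and after a short delay the arrow is registered through the player character's HUD.
; A one-time Interact stops the bounce, plays the plant sound, notifies the game mode, then swaps the cone for a cube and removes the arrow.
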(event `self.ReceiveBeginPlay`
  (`|ExecutionSequence`
    (:`then_0`
      (bind (_direction _offset) (`Timeline|Bouncing` :!label _label)
        (:`Update`
          (`SceneComponent.K2_AddLocalOffset` (`self.Cone`) (`KismetMathLibrary.MakeVector` 0.0 0.0 _offset) false false))))
    (:`then_1`
      (`KismetSystemLibrary.Delay` 0.5)
      (bind _asnew_player_controller (cast `/Game/Blueprints/NewPlayerController` (`GameplayStatics.GetPlayerController` 0)))
      (bind _asbp_third_person_character (cast `/Game/Blueprints/BP_ThirdPersonCharacter` (`/Game/Blueprints/NewPlayerController.TargetCharacter` _asnew_player_controller)))
      (bind _result (`/Game/Blueprints/UI/Minimap/MinimapWidget.AddArrow` (`/Game/Blueprints/UI/BP_Hud.MinimapWidget` (`/Game/Blueprints/BP_ThirdPersonCharacter.Hud REF` _asbp_third_person_character)) true (make `Color` 0 1 0 1) self)))))

(event `Interact`
  (`/Engine/EditorBlueprintResources/StandardMacros.DoOnce` false
    (:`Completed`
      (`|ExecutionSequence`
        (:`then_0`
          (goto _label :!via `Stop`))
        (:`then_1`
          (`GameplayStatics.PlaySoundAtLocation` "/Game/Audio/PlantBomb.PlantBomb" (`self.K2_GetActorLocation`) (struct) 1.0 1.0 0.0 null null null null)
          (bind _asbp_third_person_game_mode (cast `/Game/Blueprints/BP_ThirdPersonGameMode` (`GameplayStatics.GetGameMode`)))
          (`/Game/Blueprints/BP_ThirdPersonGameMode.BombPlanted` _asbp_third_person_game_mode)
          (`SceneComponent.SetVisibility` (`self.Cube`) true false)
          (`SceneComponent.SetVisibility` (`self.Cone`) false false)
          (`Widget.RemoveFromParent` (stale `self.ReceiveBeginPlay` _result)))))))

(fn `UserConstructionScript`)