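; Exit door objective that ends the game in victory when the player interacts after the game mode unlocks the exit.
; Interact shows and reuses a victory widget with sound, switches to UI-only input, pauses, marks the game over and turns off the HUD.
; DisplayMarker reveals a cone, moved by a timeline that also calls AddArrow on every update to mark the door on the minimap.
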(event `Interact`
  (bind _returnvalue (`GameplayStatics.GetPlayerController` 0))
  (bind _victorymenu (`self.VictoryMenu`))
  (bind _asbp_third_person_game_mode (cast `/Game/Blueprints/BP_ThirdPersonGameMode` (`GameplayStatics.GetGameMode`)))
  (if (`/Game/Blueprints/BP_ThirdPersonGameMode.unlockExit` _asbp_third_person_game_mode)
    (`/Engine/EditorBlueprintResources/StandardMacros.IsValid` (`self.VictoryMenu`)
      (:`Is Valid`
        _)
      (:`Is Not Valid`
        (bind _returnvalue_2 (`|CreateWidget` "/Game/Blueprints/UI/BP_Victory.BP_Victory_C"))
        (set `self.VictoryMenu` _returnvalue_2)))
    (`WidgetBlueprintLibrary.SetInputMode_UIOnlyEx` _returnvalue _victorymenu)
    (`UserWidget.AddToViewport` _victorymenu 0)
    (`/Game/Blueprints/UI/BP_Victory.PlayVictorySound` _victorymenu)
    (set `PlayerController.bShowMouseCursor` true _returnvalue)
    (`GameplayStatics.SetGamePaused` true)
    (bind _asbp_third_person_game_mode_2 (cast `/Game/Blueprints/BP_ThirdPersonGameMode` (`GameplayStatics.GetGameMode`)))
    (set `/Game/Blueprints/BP_ThirdPersonGameMode.gameInProgress` false _asbp_third_person_game_mode_2)
    ;[1 1 1] Turn Hud Off
    (bind _asbp_third_person_character (cast `/Game/Blueprints/BP_ThirdPersonCharacter` (`GameplayStatics.GetPlayerCharacter` 0)))
    (`/Game/Blueprints/BP_ThirdPersonCharacter.Create/ Set Hud` _asbp_third_person_character false)))

(event `DisplayMarker`
  (`SceneComponent.SetVisibility` (`self.Cone`) true false)
  (bind (_direction _offset) (`Timeline|Timeline_0`)
    (:`Update`
      (`SceneComponent.K2_AddLocalOffset` (`self.Cone`) (`KismetMathLibrary.MakeVector` 0.0 0.0 _offset) false false)
      (bind _asnew_player_controller (cast `/Game/Blueprints/NewPlayerController` (`GameplayStatics.GetPlayerController` 0)))
      (bind _asbp_third_person_character (cast `/Game/Blueprints/BP_ThirdPersonCharacter` (`/Game/Blueprints/NewPlayerController.TargetCharacter` _asnew_player_controller)))
      (`/Game/Blueprints/UI/Minimap/MinimapWidget.AddArrow` (`/Game/Blueprints/UI/BP_Hud.MinimapWidget` (`/Game/Blueprints/BP_ThirdPersonCharacter.Hud REF` _asbp_third_person_character)) true (make `Color` 0 1 0 1) self))))

(fn `UserConstructionScript`)